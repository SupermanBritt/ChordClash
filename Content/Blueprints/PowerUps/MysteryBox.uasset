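; Mystery box that spawns and assigns a power-up to each of the two players on BeginPlay and GiveOutPowerups.
; GivePlayerPowerUp picks one of seven probability rows from the players' health gap, then rolls a weighted index.
; That roll is currently unused: ManualOverride selects among six power-up classes, hardcoded to Shield for Player 1 and PiercingWail for Player 2.
; The spawned actor appears at a fixed per-player transform and passes to SetPowerup.
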(event Custom|GetPlayerReference
  ;[1 1 1] Gets a reference to the players
  (bind _outactors (Actor|GetAllActorsOfClass "/Game/Blueprints/Player1Pawn_Blueprint.Player1Pawn_Blueprint_C"))
  (Variables|Default|SetPlayer1 (Utilities|Array|Get(acopy) _outactors))
  (bind _outactors_2 (Actor|GetAllActorsOfClass "/Game/Blueprints/Player2Pawn_Blueprint.Player2Pawn_Blueprint_C"))
  (Variables|Default|SetPlayer2 (Utilities|Array|Get(acopy) _outactors_2)))

(event Custom|GiveOutPowerups
  (CallFunction|GivePlayerPowerUp true 3)
  (CallFunction|GivePlayerPowerUp false 1))

(event EventBeginPlay
  (CallFunction|GetPlayerReference)
  (Variables|Default|SetMaxHealth (Variables|/Game/Blueprints/Player1Pawn_Blueprint.Player1Pawn_Blueprint_C|GetMaxHealth (Variables|Default|GetPlayer1)))
  (CallFunction|GivePlayerPowerUp true 3)
  (CallFunction|GivePlayerPowerUp false 1))

(event Collision|EventActorBeginOverlap
  (params (OtherActor :type Actor%20Object%20Reference)))

(event EventTick
  (params (DeltaSeconds :type Float%20%28single-precision%29)))

(fn ConstructionScript)

(fn GivePlayerPowerUp
  (params (IsPlayer1 :type Boolean) (Manual%20Override :type Integer))
  (bind _player1 (Variables|Default|GetPlayer1))
  (bind _player2 (Variables|Default|GetPlayer2))
  (bind _maxhealth (Variables|Default|GetMaxHealth))
  (bind _health (Variables|/Game/Blueprints/Player1Pawn_Blueprint.Player1Pawn_Blueprint_C|GetHealth _player1))
  (bind _health_2 (Variables|/Game/Blueprints/Player2Pawn_Blueprint.Player2Pawn_Blueprint_C|GetHealth _player2))
  (bind _returnvalue (- _health _health_2))
  (bind _returnvalue_2 (/ _returnvalue _maxhealth))
  (Variables|Default|SetTransform (Math|Transform|SelectTransform (Math|Transform|MakeTransform "-670.000000,-4710.000000,370.000000" "0, 0, 0" "0.250000,0.250000,0.250000") (Math|Transform|MakeTransform "-670.000000,-5100.000000,370.000000" "0, 0, 0" "0.250000,0.250000,0.250000") IsPlayer1))
  (if IsPlayer1
    (Variables|Default|SetPercentDiff (* _returnvalue_2 -1.0)) ; Player 1
    (else
      (Variables|Default|SetPercentDiff _returnvalue_2) ; Player2
    ))
  ;[1 1 1] If/Else Block For Determining Which Probability to Use
  (if (< (Variables|Default|GetPercentDiff) -0.7)
    (Variables|Default|SetProbabilityIndex 0)
    (elif (< (Variables|Default|GetPercentDiff) -0.4)
      (Variables|Default|SetProbabilityIndex 1)
      (elif (< (Variables|Default|GetPercentDiff) -0.1)
        (Variables|Default|SetProbabilityIndex 2)
        (elif (< (Variables|Default|GetPercentDiff) 0.1)
          (Variables|Default|SetProbabilityIndex 3)
          (elif (< (Variables|Default|GetPercentDiff) 0.4)
            (Variables|Default|SetProbabilityIndex 4)
            (elif (< (Variables|Default|GetPercentDiff) 0.7)
              (Variables|Default|SetProbabilityIndex 5)
              (else
                (Variables|Default|SetProbabilityIndex 6))))))))
  (CallFunction|CalculateRandomBasedonSixFloats (Utilities|Array|Get(acopy) (Variables|Default|GetPowerupProbability) (Variables|Default|GetProbabilityIndex)))
  (switch int (Class|KismetSystemLibrary|MakeLiteralInteger Manual%20Override)
    (:0
      (bind _returnvalue_3 (Game|SpawnActorfromClass "/Game/Blueprints/PowerUps/ComboLock.ComboLock_C" (Variables|Default|GetTransform) "Undefined" "MultiplyWithRoot" 0 0))
      (Variables|Default|SetPowerup _returnvalue_3))
    (:1
      (bind _returnvalue_4 (Game|SpawnActorfromClass "/Game/Blueprints/PowerUps/PiercingWail.PiercingWail_C" (Variables|Default|GetTransform) "Undefined" "MultiplyWithRoot" 0 0))
      (Variables|Default|SetPowerup _returnvalue_4))
    (:2
      (bind _returnvalue_5 (Game|SpawnActorfromClass "/Game/Blueprints/PowerUps/MedKit.MedKit_C" (Variables|Default|GetTransform) "Undefined" "MultiplyWithRoot" 0 0))
      (Variables|Default|SetPowerup _returnvalue_5))
    (:3
      (bind _returnvalue_6 (Game|SpawnActorfromClass "/Game/Blueprints/PowerUps/Shield.Shield_C" (Variables|Default|GetTransform) "Undefined" "MultiplyWithRoot" 0 0))
      (Variables|Default|SetPowerup _returnvalue_6))
    (:4
      (bind _returnvalue_7 (Game|SpawnActorfromClass "/Game/Blueprints/PowerUps/AutoPerfect.AutoPerfect_C" (Variables|Default|GetTransform) "Undefined" "MultiplyWithRoot" 0 0))
      (Variables|Default|SetPowerup _returnvalue_7))
    (:5
      (bind _returnvalue_8 (Game|SpawnActorfromClass "/Game/Blueprints/PowerUps/Freeze.Freeze_C" (Variables|Default|GetTransform) "Undefined" "MultiplyWithRoot" 0 0))
      (Variables|Default|SetPowerup _returnvalue_8)))
  (if IsPlayer1
    (Default|SetPowerup (Variables|Default|GetPlayer1) (Variables|Default|GetPowerup))
    (else
      (Default|SetPowerup (Variables|Default|GetPlayer2) (Variables|Default|GetPowerup)))))

(fn CalculateRandomBasedonSixFloats
  (params (Probabilites :type Float%20Array%20Structure))
  (LocalVariables|SetRandomValue (Math|Conversions|ToFloat(Integer) (Math|Random|RandomInteger 1000)))
  (for (_array_element _array_index) (Utilities|Struct|BreakFloatArray Probabilites)
    ;[1 1 1] IndexRandom += PowerupProbabilities[i] * 10
    (bind _output_get (LocalVariables|SetIndexRandom (+ (* _array_element 1e+01) (LocalVariables|GetIndexRandom))))
    (if (< (LocalVariables|GetRandomValue) _output_get)
      (return _array_index)))
  (return -1) ; Error
)