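; Pawn Blueprint for player two that stores the player's character, skill, song and powerup selections.
; Setup and SetSong take enum values from the level blueprint when menu options are picked or the song changes, while SetPowerup stores a new powerup.
; Each setter prints its value to screen for debugging, though SetSong labels its message "Player1" rather than "Player2".
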(fn ConstructionScript)

(fn Setup
  (params (Character :type CharactersEnum%20Enum :default "NewEnumerator0") (Skill :type SkillsEnum%20Enum :default "NewEnumerator0"))
  ;[1 1 1] The Setup function sets the character enum and skill enum values to be the corresponding parameters of the function. This gets called in the level blueprint after the options have been selected in the menu.
  (Variables|Default|SetCharacter Character)
  (Variables|Default|SetSkill Skill)
  (Development|PrintString (Utilities|String|Append "Player2:" (Utilities|String|EnumtoString (Variables|Default|GetSkill)) (Utilities|String|EnumtoString (Variables|Default|GetCharacter))) true true "(R=1.000000,G=0.000000,B=0.000000,A=1.000000)" 1e+02))

(fn SetSong
  (params (Song :type SongsEnum%20Enum :default "NewEnumerator0"))
  ;[1 1 1] The SetSong function sets the song enum value to be the corresponding parameters of the function. This gets called in the level blueprint anytime the player changes their selected song.
  (Variables|Default|SetSong Song)
  (Development|PrintString (Utilities|String|Append "Player1:" (Utilities|String|EnumtoString (Variables|Default|GetSong))) true true "(R=1.000000,G=0.000000,B=0.000000,A=1.000000)" 1e+02))

(fn SetPowerup
  (params (newPowerup :type Powerup%20Object%20Reference))
  (bind _output_get (Variables|Default|SetPowerup newPowerup))
  (Development|PrintString (Utilities|GetDisplayName _output_get) true true "(R=0.000000,G=0.660000,B=1.000000,A=1.000000)" 1e+01))