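; SingerManager is an actor Blueprint that switches which player's singer sequence is active based on the two players' health.
; The SwitchSinger event activates the sequence of the player with more health and deactivates the other's, or activates both on a tie.
; Activation toggles SetIsActive on the first section of the first track that has one in each player's SingerSequence.
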(event Custom|SwitchSinger
  (bind _player1 (Variables|Default|GetPlayer1))
  (bind _player2 (Variables|Default|GetPlayer2))
  (bind _health (Variables|/Game/Blueprints/Player1Pawn_Blueprint.Player1Pawn_Blueprint_C|GetHealth _player1))
  (bind _health_2 (Variables|/Game/Blueprints/Player2Pawn_Blueprint.Player2Pawn_Blueprint_C|GetHealth _player2))
  (bind _singersequence (Variables|/Game/Blueprints/Player1Pawn_Blueprint.Player1Pawn_Blueprint_C|GetSingerSequence _player1))
  (bind _singersequence_2 (Variables|/Game/Blueprints/Player2Pawn_Blueprint.Player2Pawn_Blueprint_C|GetSingerSequence _player2))
  (if (> _health _health_2)
    (CallFunction|ActivateSequence _singersequence)
    (CallFunction|DeactivateSequence _singersequence_2)
    (elif (== _health _health_2)
      (CallFunction|ActivateSequence _singersequence)
      (CallFunction|ActivateSequence _singersequence_2)
      (else
        (CallFunction|DeactivateSequence _singersequence)
        (CallFunction|ActivateSequence _singersequence_2)))))

(event EventBeginPlay)

(event Collision|EventActorBeginOverlap
  (params (OtherActor :type Actor%20Object%20Reference)))

(event EventTick
  (params (DeltaSeconds :type Float%20%28single-precision%29)))

(fn ConstructionScript)

(fn ActivateSequence
  (params (PlayerSequence :type Movie%20Scene%20Sequence%20Object%20Reference))
  (bind _seqsection (CallFunction|GetSection PlayerSequence))
  (Class|MovieSceneSection|SetIsActive _seqsection true)
  (return))

(fn DeactivateSequence
  (params (PlayerSequence :type Movie%20Scene%20Sequence%20Object%20Reference))
  (bind _seqsection (CallFunction|GetSection PlayerSequence))
  (Class|MovieSceneSection|SetIsActive _seqsection false)
  (return))

(fn GetSection
  (params (PlayerSequence :type Movie%20Scene%20Sequence%20Object%20Reference))
  (bind _returnvalue (Class|MovieSceneSequenceExtensions|GetTracks PlayerSequence))
  (for _array_element _returnvalue
    (bind _returnvalue_2 (Class|MovieSceneTrackExtensions|GetSections _array_element))
    (for _array_element_2 _returnvalue_2
      (return _array_element_2))))