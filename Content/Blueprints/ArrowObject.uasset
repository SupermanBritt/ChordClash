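; Falling arrow note for a four-lane, rhythm-style game, with a one-in-ten chance of becoming a mystery note.
; On BeginPlay it sets a mystery or lane-direction sprite, then scrolls it down through chained MoveComponentTo calls.
; Move durations scale with Offset to keep a constant speed.
; At the first endpoint it calls RemoveFromQueue with its lane and spawn number, then keeps falling and destroys itself.
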(event EventBeginPlay
  (bind _offset (Variables|Default|GetOffset))
  (bind _arrowsprite (Variables|Default|GetArrowSprite))
  (if (== (Math|Random|RandomIntegerinRange 1 10) 6)
    (Variables|Default|SetisMystery true)
    (Rendering|Components|Sprite|SetSprite (Variables|Default|GetArrowSprite) "/Game/2DSprites/mystery_Sprite.mystery_Sprite")
    (else
      (switch string (Variables|Default|GetLane)
        (:1
          (Rendering|Components|Sprite|SetSprite (Variables|Default|GetArrowSprite) "/Game/2DSprites/leftArrow_Sprite.leftArrow_Sprite"))
        (:2
          (Rendering|Components|Sprite|SetSprite (Variables|Default|GetArrowSprite) "/Game/2DSprites/downArrow_Sprite.downArrow_Sprite"))
        (:3
          (Rendering|Components|Sprite|SetSprite (Variables|Default|GetArrowSprite) "/Game/2DSprites/upArrow_Sprite.upArrow_Sprite"))
        (:4
          (Rendering|Components|Sprite|SetSprite (Variables|Default|GetArrowSprite) "/Game/2DSprites/rightArrow_Sprite.rightArrow_Sprite")))))
  (if (>= _offset 0.0)
    (Components|MoveComponentTo _arrowsprite (Math|Vector|MakeVector 0.0 0.0 (- 0.0 (* (Variables|Default|GetOffset) 1e+01))) "0, 0, 0" false false (* _offset 0.02857) false)
    (Components|MoveComponentTo _arrowsprite (Math|Vector|MakeVector 0.0 0.0 (- -8.5e+02 (* (Variables|Default|GetOffset) 1e+01))) "0, 0, 0" false false 2.428571 false)
    (else
      (Components|MoveComponentTo (Variables|Default|GetArrowSprite) (Math|Vector|MakeVector 0.0 0.0 (- -8.5e+02 (* (Variables|Default|GetOffset) 1e+01))) "0, 0, 0" false false (- 2.428571 (* (Variables|Default|GetOffset) -0.02857)) false)))
  (Default|CallRemovefromQueue (Variables|Default|GetLane) (Variables|Default|GetSpawnNum))
  (Components|MoveComponentTo _arrowsprite (Math|Vector|MakeVector 0.0 0.0 (- -1.55e+03 (* (Variables|Default|GetOffset) 1e+01))) "0, 0, 0" false false 2.0 false)
  (Utilities|FlowControl|Delay 0.2)
  (Actor|DestroyActor))

(event Collision|EventActorBeginOverlap
  (params (OtherActor :type Actor%20Object%20Reference)))

(event EventTick
  (params (DeltaSeconds :type Float%20%28single-precision%29)))

(fn ConstructionScript)