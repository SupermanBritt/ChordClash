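; Player 1's pawn in a two-player music game, holding health, character, skill, song choice and briefly buffered directional key presses.
; It carries one powerup at a time; UsePowerup dispatches on its type to self buffs, healing, or attacks on the Player 2 pawn that shields block.
; Timers end temporary effects and Call events announce state changes.
; ChangeHealth clamps health, flags zero, and triggers damage-scaled particles and character-specific hit sounds.
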(event Custom|UseComboLock
  (Variables|Default|SethasComboLock true)
  (Default|CallP1ComboLock)
  (Audio|PlaySound2D "/Game/Sounds/Powerups/combolock.combolock" 1.0 1.0 0.0 0 0))

(event Custom|UsePiercingWail
  (if (Variables|/Game/Blueprints/Player2Pawn_Blueprint.Player2Pawn_Blueprint_C|GethasShield (Utilities|Array|Get(acopy) (stale EventBeginPlay _outactors)))
    (Audio|PlaySound2D "/Game/Sounds/Powerups/hitshield.hitshield" 1.0 1.0 0.0 0 0)
    (else
      (Default|ChangeHealth (Utilities|Array|Get(acopy) (stale EventBeginPlay _outactors)) -5e+01)
      (Audio|PlaySound2D "/Game/Sounds/Powerups/wail.wail" 1.0 1.0 0.0 0 0))))

(event Custom|SetPressUp
  (params (Press%20Up :type Boolean))
  (Variables|Default|SetPressUp Press%20Up)
  (Utilities|FlowControl|Delay 0.1)
  (Variables|Default|SetcurrentKey "up")
  (Utilities|FlowControl|Delay 1.0)
  (Variables|Default|SetcurrentKey "none"))

(event Custom|SetPressLeft
  (params (Press%20Left :type Boolean))
  (Variables|Default|SetPressLeft Press%20Left)
  (Utilities|FlowControl|Delay 0.1)
  (Variables|Default|SetcurrentKey "left")
  (Utilities|FlowControl|Delay 1.0)
  (Variables|Default|SetcurrentKey "none"))

(event Custom|SetPressDown
  (params (Press%20Down :type Boolean))
  (Variables|Default|SetPressDown Press%20Down)
  (Utilities|FlowControl|Delay 0.1)
  (Variables|Default|SetcurrentKey "down")
  (Utilities|FlowControl|Delay 1.0)
  (Variables|Default|SetcurrentKey "none"))

(event Custom|UseMedKit
  (CallFunction|ChangeHealth 5e+01)
  (Audio|PlaySound2D "/Game/Sounds/Powerups/heal.heal" 1.0 1.0 0.0 0 0))

(event Custom|UseShield
  (Variables|Default|SethasShield true)
  (Default|CallP1Shielded)
  (Utilities|Time|SetTimerbyEvent (delegate Custom|TurnOffShield) 5.0)
  (Audio|PlaySound2D "/Game/Sounds/Powerups/shield.shield" 1.0 1.0 0.0 0 0))

(event Custom|UseAutoPerfect
  (Variables|Default|SetisAutoPerfect true)
  (Default|CallP1AutoP)
  (Utilities|Time|SetTimerbyEvent (delegate Custom|TurnOffAutoPerfect) 3.0)
  (Audio|PlaySound2D "/Game/Sounds/Powerups/autoperfect.autoperfect" 1.0 1.0 0.0 0 0))

(event Custom|UseFreeze
  (if (Variables|/Game/Blueprints/Player2Pawn_Blueprint.Player2Pawn_Blueprint_C|GethasShield (Utilities|Array|Get(acopy) (stale EventBeginPlay _outactors)))
    (Audio|PlaySound2D "/Game/Sounds/Powerups/hitshield.hitshield" 1.0 1.0 0.0 0 0)
    (else
      (Variables|/Game/Blueprints/Player2Pawn_Blueprint.Player2Pawn_Blueprint_C|SetisFrozen (Utilities|Array|Get(acopy) (stale EventBeginPlay _outactors)) true)
      (Default|CallP2Frozen)
      (Utilities|Time|SetTimerbyEvent (delegate Custom|UnFreezeOpponent) 3.0)
      (Audio|PlaySound2D "/Game/Sounds/Powerups/freeze.freeze" 1.0 1.0 0.0 0 0))))

(event Custom|UnFreezeOpponent
  (Variables|/Game/Blueprints/Player2Pawn_Blueprint.Player2Pawn_Blueprint_C|SetisFrozen (Utilities|Array|Get(acopy) (stale EventBeginPlay _outactors)) false)
  (Audio|PlaySound2D "/Game/Sounds/Powerups/unfreeze.unfreeze" 1.0 1.0 0.0 0 0))

(event Custom|TurnOffAutoPerfect
  (Variables|Default|SetisAutoPerfect false)
  (Audio|PlaySound2D "/Game/Sounds/Powerups/autoperfectend.autoperfectend" 1.0 1.0 0.0 0 0))

(event Custom|TurnOffShield
  (Variables|Default|SethasShield false)
  (Audio|PlaySound2D "/Game/Sounds/Powerups/unshield.unshield" 1.0 1.0 0.0 0 0))

(event Custom|SetPressRight
  (params (pressRight :type Boolean))
  (Variables|Default|SetPressRight pressRight)
  (Utilities|FlowControl|Delay 0.1)
  (Variables|Default|SetcurrentKey "right")
  (Utilities|FlowControl|Delay 1.0)
  (Variables|Default|SetcurrentKey "none"))

(event EventBeginPlay
  (Variables|Default|SetHealth (Variables|Default|GetMaxHealth))
  (CallFunction|SetPowerup)
  (bind _outactors (Actor|GetAllActorsOfClass "/Game/Blueprints/Player2Pawn_Blueprint.Player2Pawn_Blueprint_C"))
  (Variables|/Game/Blueprints/Player2Pawn_Blueprint.Player2Pawn_Blueprint_C|SetMaxHealth (Utilities|Array|Get(acopy) _outactors) (Variables|Default|GetMaxHealth)))

(fn ConstructionScript)

(fn Setup
  (params (Character :type CharactersEnum%20Enum :default "NewEnumerator0") (Skill :type SkillsEnum%20Enum :default "NewEnumerator0"))
  ;[1 1 1] The Setup function sets the character enum and skill enum values to be the corresponding parameters of the function. This gets called in the level blueprint after the options have been selected in the menu.
  (Variables|Default|SetCharacter Character)
  (Variables|Default|SetSkill Skill)
  (Development|PrintString (Utilities|String|Append "Player1:" (Utilities|String|EnumtoString (Variables|Default|GetSkill)) (Utilities|String|EnumtoString (Variables|Default|GetCharacter))) true true "(R=1.000000,G=0.000000,B=0.000000,A=1.000000)" 1e+02))

(fn SetSong
  (params (Song :type SongsEnum%20Enum :default "NewEnumerator0"))
  ;[1 1 1] The SetSong function sets the song enum value to be the corresponding parameters of the function. This gets called in the level blueprint anytime the player changes their selected song.
  (Variables|Default|SetSong Song)
  (Development|PrintString (Utilities|String|Append "Player1:" (Utilities|String|EnumtoString (Variables|Default|GetSong))) true true "(R=1.000000,G=0.000000,B=0.000000,A=1.000000)" 1e+02))

(fn SetPowerup
  (params (NewPowerup :type Powerup%20Object%20Reference))
  (if (Utilities|IsValid (Variables|Default|GetPowerup))
    (Actor|DestroyActor NewPowerup)
    (Audio|PlaySound2D "/Game/Sounds/Powerups/haspowerupalready.haspowerupalready" 1.0 1.0 0.0 0 0)
    (else
      (bind _output_get (Variables|Default|SetPowerup NewPowerup))
      (if (Utilities|IsValid _output_get)
        (Audio|PlaySound2D "/Game/Sounds/Powerups/getpowerup.getpowerup" 1.0 1.0 0.0 0 0)))))

(fn UsePowerup
  (if (Utilities|IsValid (Variables|Default|GetPowerup))
    (switch Utilities|FlowControl|Switch|SwitchonPowerupEnum (Variables|/Game/Blueprints/PowerUps/Powerup.Powerup_C|GetType (Variables|Default|GetPowerup))
      (:NewEnumerator0
        (CallFunction|UseComboLock))
      (:NewEnumerator1
        (CallFunction|UsePiercingWail))
      (:NewEnumerator2
        (CallFunction|UseMedKit))
      (:NewEnumerator3
        (CallFunction|UseShield))
      (:NewEnumerator4
        (CallFunction|UseAutoPerfect))
      (:NewEnumerator5
        (CallFunction|UseFreeze)))
    (Actor|DestroyActor (Variables|Default|GetPowerup))))

(fn ChangeHealth
  (params (delta :type Float%20%28double-precision%29))
  (if (> (+ delta (Variables|Default|GetHealth)) (Variables|Default|GetMaxHealth))
    (Variables|Default|SetHealth (Variables|Default|GetMaxHealth))
    (else
      (CallFunction|PlayHitSound delta)
      (if (< (+ delta (Variables|Default|GetHealth)) 0.0)
        (Variables|Default|SetHealth 0.0)
        (Variables|Default|SetHealthZero true)
        (Default|CallP1Health0)
        (elif (not (Variables|Default|GetHealthZero))
          (Variables|Default|SetHealth (+ delta (Variables|Default|GetHealth))))))))

(fn ResetPlayer
  (Variables|Default|SetHealth (Variables|Default|GetMaxHealth))
  (if (Utilities|IsValid (Variables|Default|GetPowerup))
    (Actor|DestroyActor (Variables|Default|GetPowerup)))
  (Variables|Default|SethasShield false)
  (Variables|Default|SethasComboLock false)
  (Variables|Default|SetisAutoPerfect false)
  (Variables|Default|SetisFrozen false)
  (Variables|Default|SetHealthZero false))

(fn PlayHitSound
  (params (Delta :type Float%20%28double-precision%29))
  (if (!= Delta 0.0)
    (if (< Delta 0.0)
      (if (>= Delta -5.0)
        (Niagara|SpawnSystematLocation "/Game/Particles/Dmg_1.Dmg_1" (Transformation|GetActorLocation) "0, 0, 0" "1.000000,1.000000,1.000000" true true "AutoRelease")
        (switch Utilities|FlowControl|Switch|SwitchonCharactersEnum (Variables|Default|GetCharacter)
          (:NewEnumerator0
            (Audio|PlaySound2D "/Game/Sounds/HurtSounds/beatheadweakhit.beatheadweakhit" 1.0 1.0 0.0 0 0))
          (:NewEnumerator1
            (Audio|PlaySound2D "/Game/Sounds/HurtSounds/bunnygirlweakhit.bunnygirlweakhit" 1.0 1.0 0.0 0 0)))
        (elif (>= 0.0 -2e+01)
          (Niagara|SpawnSystematLocation "/Game/Particles/Dmg_2.Dmg_2" (Transformation|GetActorLocation) "0, 0, 0" "1.000000,1.000000,1.000000" true true "AutoRelease")
          (if (>= Delta -15.0)
            (switch Utilities|FlowControl|Switch|SwitchonCharactersEnum (Variables|Default|GetCharacter)
              (:NewEnumerator0
                (Audio|PlaySound2D "/Game/Sounds/HurtSounds/beatheadmediumhit.beatheadmediumhit" 1.0 1.0 0.0 0 0))
              (:NewEnumerator1
                (Audio|PlaySound2D "/Game/Sounds/HurtSounds/bunnygirlmediumhit.bunnygirlmediumhit" 1.0 1.0 0.0 0 0)))
            (else
              (switch Utilities|FlowControl|Switch|SwitchonCharactersEnum (Variables|Default|GetCharacter) :!label _label
                (:NewEnumerator0
                  (Audio|PlaySound2D "/Game/Sounds/HurtSounds/beatheadstronghit.beatheadstronghit" 1.0 1.0 0.0 0 0))
                (:NewEnumerator1
                  (Audio|PlaySound2D "/Game/Sounds/HurtSounds/bunnygirlstronghit.bunnygirlstronghit" 1.0 1.0 0.0 0 0)))))
          (else
            (Niagara|SpawnSystematLocation "/Game/Particles/Dmg_3.Dmg_3" (Transformation|GetActorLocation) "0, 0, 0" "1.000000,1.000000,1.000000" true true "AutoRelease")
            (goto _label))))
      (elif (<= Delta 1e+01)
        (Niagara|SpawnSystematLocation "/Game/Particles/Heal_1.Heal_1" (Transformation|GetActorLocation) "0, 0, 0" "1.000000,1.000000,1.000000" true true "AutoRelease")
        (else
          (Niagara|SpawnSystematLocation "/Game/Particles/Heal_2.Heal_2" (Transformation|GetActorLocation) "0, 0, 0" "1.000000,1.000000,1.000000" true true "AutoRelease"))))))